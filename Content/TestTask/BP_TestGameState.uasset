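; Test game state that acts as the server-side hub for player chat, keeping a fixed-size message history.
; SendMessage runs only with authority and builds a message from the text, sender's player name and current hour and minute.
; PushMessageCircular writes it into the pre-sized ChatHistory as a ring buffer.
; The entry at the returned index then goes to every actor implementing the ChatListener interface.
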(event EventSendMessage
  (params (MessageText :type String) (Caller :type Player%20State%20Object%20Reference))
  (bind _returnvalue (Math|DateTime|Now))
  ;[1 1 1] On message sent add received message to array and then make interface call to all listeners
  (Networking|SwitchHasAuthority
    (:Authority
      (bind _index (Utilities|PushMessageCircular (Utilities|Struct|MakeMessage (Utilities|Struct|MakeTimecode (Class|KismetMathLibrary|GetHour _returnvalue) (Class|KismetMathLibrary|GetMinute _returnvalue)) (PlayerState|GetPlayerName Caller) MessageText)))
      (bind _outactors (Actor|GetAllActorswithInterface "/Game/TestTask/Chat/ChatListener.ChatListener_C"))
      (for _array_element _outactors
        (Class|ChatListener|OnMessageReceive(Message) _array_element (Utilities|Array|Get(acopy) (Variables|Default|GetChatHistory) _index))))))

(event EventBeginPlay
  (Utilities|Array|Resize (Variables|Default|GetChatHistory) (Variables|Default|GetMaxMessages)))

(fn ConstructionScript)

(fn PushMessage
  (params (Message :type Message%20Structure%20%28by%20ref%29)))