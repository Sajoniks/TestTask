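; Test player controller that carries text chat between its client and the server.
; The T key opens chat on BP_HUD, and a server RPC passes outgoing text with the PlayerState to the GameState through the ChatOperator interface.
; Received messages are forwarded to the owning client by RPC, which fires the OnChatMessageReceived dispatcher.
; SetPlayerName requests a name change from the GameMode.
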(event Custom|Server_SendMessage
  (params (MessageText :type String))
  (bind _returnvalue (Game|GetGameState))
  ;[1 1 1] RPC asks to send message
  (if (Utilities|DoesObjectImplementInterface _returnvalue "/Game/TestTask/Chat/ChatOperator.ChatOperator_C")
    (Class|ChatOperator|SendMessage(Message) _returnvalue MessageText (Variables|GetPlayerState))))

(event Custom|Client_MessageReceived
  (params (Message :type Message%20Structure))
  ;[1 1 1] Replicate received message to owning client controller
  (Default|CallOnChatMessageReceived Message))

(event EventOnMessageReceive
  (params (Message :type Message%20Structure))
  ;[1 1 1] Called when message received on server
  (CallFunction|ClientMessageReceived Message))

(event Input|KeyboardEvents|T
  (params (Key :type Key%20Structure :default "None"))
  (:Pressed
    (bind _asbp_hud (Utilities|Casting|CastToBP_HUD (HUD|GetHUD)))
    (Default|OpenChat _asbp_hud)))

(fn ConstructionScript)

(fn SetPlayerName
  (params (Name :type String))
  (Class|GameModeBase|ChangeName (Game|GetGameMode) self Name true))